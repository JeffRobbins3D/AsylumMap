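; Interactive front door Blueprint that the player swings open and closed, or rattles when it is locked.
; A Box overlap enables and disables player input, so Interact only works while in range.
; Interact either plays a locked-shake timeline or plays and reverses a timeline that rotates the Arrow toward OpenAngle.
; BeginPlay sets the swing direction from ReverseOpen, and DoorClosed follows the timeline's value to choose between opening and closing.
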(event `self.Box.OnComponentBeginOverlap`
  (params (OverlappedComponent :type "PrimitiveComponent Object Reference") (OtherActor :type "Actor Object Reference") (OtherComp :type "PrimitiveComponent Object Reference") (OtherBodyIndex :type Integer) (bFromSweep :type Boolean) (SweepResult :type "HitResult Structure (by ref)"))
  ;[1 1 1] Events
  ;[1 1 1] Enable input
  (`self.EnableInput` (`GameplayStatics.GetPlayerController` 0)))

(event `self.Box.OnComponentEndOverlap`
  (params (OverlappedComponent :type "PrimitiveComponent Object Reference") (OtherActor :type "Actor Object Reference") (OtherComp :type "PrimitiveComponent Object Reference") (OtherBodyIndex :type Integer))
  ;[1 1 1] Events
  ;[1 1 1] Enable input
  (`self.DisableInput` (`GameplayStatics.GetPlayerController` 0)))

(event `InputAction|Interact`
  (params (Key :type "Key Structure" :default "AnyKey"))
  ;[1 1 1] Events
  (:`Pressed`
    ;[1 1 1] Locked check
    (if (`self.IsLocked`)
      ;[1 1 1] Locked animation
      (bind (_direction _doorlockedrotate) (`Timeline|Timeline_1` :!via `PlayFromStart`)
        (:`Update`
          (`SceneComponent.K2_SetRelativeRotation` (`self.Arrow`) (`KismetMathLibrary.MakeRotator` 0.0 0.0 _doorlockedrotate) false false)))
      (else
        ;[1 1 1] Unlocked animation
        (if (`self.DoorClosed`)
          (bind (_direction_2 _doorrotate) (`Timeline|Timeline_0` :!label _label)
            (:`Update`
              (`SceneComponent.K2_SetRelativeRotation` (`self.Arrow`) (`KismetMathLibrary.RLerp` (struct) (`KismetMathLibrary.MakeRotator` 0.0 0.0 (`self.OpenAngle`)) _doorrotate) false false)
              (set `self.DoorClosed` (== _doorrotate 0.0))))
          (else
            (goto _label :!via `Reverse`)))))))

(event `self.ReceiveBeginPlay`
  ;[1 1 1] Events
  ;[1 1 1] Set open direction (normal/reverse)
  (if (`self.ReverseOpen`)
    (set `self.OpenAngle` -90.0)
    (else
      (set `self.OpenAngle` 90.0))))

(fn `UserConstructionScript`)