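; Interactable window Blueprint whose bottom frame slides vertically between a closed and an open height.
; Overlapping the Box enables input for the first player controller, and leaving it disables input.
; Interact plays or reverses a timeline based on IsOpen, lerping the frame's relative Z position.
; IsOpen is updated during the slide and stays true while the timeline alpha is above zero.
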(event `self.ReceiveBeginPlay`
  ;[1 1 1] Set start and end locations for bottom window
  (bind _output_get (set `self.BottomWindowStartZ` 10.0))
  (set `self.BottomWindowEndZ` 95.0)
  (`SceneComponent.K2_SetRelativeLocation` (`self.BottomWindowFrame`) (`KismetMathLibrary.MakeVector` 0.0 0.0 _output_get) false false))

(event `self.Box.OnComponentBeginOverlap`
  (params (OverlappedComponent :type "PrimitiveComponent Object Reference") (OtherActor :type "Actor Object Reference") (OtherComp :type "PrimitiveComponent Object Reference") (OtherBodyIndex :type Integer) (bFromSweep :type Boolean) (SweepResult :type "HitResult Structure (by ref)"))
  ;[1 1 1] Enable input
  (`self.EnableInput` (`GameplayStatics.GetPlayerController` 0)))

(event `self.Box.OnComponentEndOverlap`
  (params (OverlappedComponent :type "PrimitiveComponent Object Reference") (OtherActor :type "Actor Object Reference") (OtherComp :type "PrimitiveComponent Object Reference") (OtherBodyIndex :type Integer))
  ;[1 1 1] Enable input
  (`self.DisableInput` (`GameplayStatics.GetPlayerController` 0)))

(event `InputAction|Interact`
  (params (Key :type "Key Structure" :default "AnyKey"))
  ;[1 1 1] Window interaction
  (:`Pressed`
    (if (stale _output_get)
      (bind (_direction _windowbottomslidealpha) (`Timeline|Timeline_0` :!via `Reverse` :!label _label)
        (:`Update`
          (`SceneComponent.K2_SetRelativeLocation` (`self.BottomWindowFrame`) (`KismetMathLibrary.VLerp` (`KismetMathLibrary.MakeVector` 0.0 0.0 (`self.BottomWindowStartZ`)) (`KismetMathLibrary.MakeVector` 0.0 0.0 (`self.BottomWindowEndZ`)) _windowbottomslidealpha) false false)
          (bind _output_get (set `self.IsOpen` (> _windowbottomslidealpha 0.0)))))
      (else
        (goto _label)))))

(fn `UserConstructionScript`)