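; Interaction_SwitchBP is an interactable on/off switch that extends a parent interaction Blueprint.
; Each Interact runs the parent logic, then flips IsActive and swaps the InteractMesh material between gold metal and basic wall.
; It updates the interaction widget's prompt to Turn Off or Turn On when the widget is valid, then calls ActivateSwitch or DeactivateSwitch to signal the new state.
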(event `self.Interact`
  (params (Character :type "/Game/FirstPerson/Blueprints/FirstPersonCharacter Object Reference"))
  ;[1 1 1] Interact with switch
  (`parent.Interact` Character)
  (if (not (`self.IsActive`))
    (set `self.IsActive` true)
    (`PrimitiveComponent.SetMaterial` (`self.InteractMesh`) 0 "/Game/StarterContent/Materials/M_Metal_Gold.M_Metal_Gold")
    (bind _interactionuiwidget (`self.InteractionUIWidget`)
      (:`then`
        (`/Game/Asylum/Blueprints/InteractionUIWBP.SetInteractDescription` _interactionuiwidget "Turn Off"))
      (:`else`
        _))
    (`self.ActivateSwitch`)
    (else
      (set `self.IsActive` false)
      (`PrimitiveComponent.SetMaterial` (`self.InteractMesh`) 0 "/Game/StarterContent/Materials/M_Basic_Wall.M_Basic_Wall")
      (bind _interactionuiwidget_2 (`self.InteractionUIWidget`)
        (:`then`
          (`/Game/Asylum/Blueprints/InteractionUIWBP.SetInteractDescription` _interactionuiwidget_2 "Turn On"))
        (:`else`
          _))
      (`self.DeactivateSwitch`))))

(fn `UserConstructionScript`
  (`parent.UserConstructionScript`))