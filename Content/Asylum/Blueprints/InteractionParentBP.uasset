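; Base Blueprint for interactable objects in the Asylum game, with a mesh, box trigger and widget prompt.
; The construction script applies configurable mesh, trigger and UI placement, and BeginPlay writes the interaction description into the widget.
; Trigger overlaps register or unregister the object with the FirstPersonCharacter.
; ToggleUI shows or hides the prompt, while Interact stores the character and only prints a debug message.
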(event `self.ReceiveBeginPlay`
  ;[1 1 1] Update UI
  (bind _asinteraction_uiwbp (cast `/Game/Asylum/Blueprints/InteractionUIWBP` (`WidgetComponent.GetUserWidgetObject` (`self.InteractUI`))))
  (bind _output_get (set `self.InteractionUIWidget` _asinteraction_uiwbp))
  (`/Game/Asylum/Blueprints/InteractionUIWBP.SetInteractDescription` _output_get (`self.InteractDescription`)))

(event `self.BoxTrigger.OnComponentBeginOverlap`
  (params (OverlappedComponent :type "PrimitiveComponent Object Reference") (OtherActor :type "Actor Object Reference") (OtherComp :type "PrimitiveComponent Object Reference") (OtherBodyIndex :type Integer) (bFromSweep :type Boolean) (SweepResult :type "HitResult Structure (by ref)"))
  ;[1 1 1] Trigger overlap
  (bind _asfirst_person_character (cast `/Game/FirstPerson/Blueprints/FirstPersonCharacter` OtherActor))
  (`/Game/FirstPerson/Blueprints/FirstPersonCharacter.AddInteraction` _asfirst_person_character self))

(event `self.BoxTrigger.OnComponentEndOverlap`
  (params (OverlappedComponent :type "PrimitiveComponent Object Reference") (OtherActor :type "Actor Object Reference") (OtherComp :type "PrimitiveComponent Object Reference") (OtherBodyIndex :type Integer))
  ;[1 1 1] Trigger overlap
  (bind _asfirst_person_character (cast `/Game/FirstPerson/Blueprints/FirstPersonCharacter` OtherActor))
  (`/Game/FirstPerson/Blueprints/FirstPersonCharacter.RemoveInteraction` _asfirst_person_character self))

(fn `InitMesh`
  ;[1 1 1] Mesh init - Set static mesh and transform
  (`StaticMeshComponent.SetStaticMesh` (`self.InteractMesh`) (`self.InteractionMeshRef`))
  (`SceneComponent.K2_SetRelativeTransform` (`self.InteractMesh`) (`self.MeshTransform`) false false))

(fn `InitTrigger`
  ;[1 1 1] Trigger init - Set scale and location
  (`SceneComponent.K2_SetRelativeLocation` (`self.BoxTrigger`) (`self.TriggerLocation`) false false)
  (`SceneComponent.SetRelativeScale3D` (`self.BoxTrigger`) (`self.TriggerScale`)))

(fn `InitUI`
  ;[1 1 1] UI Init - Set location
  (`SceneComponent.K2_SetRelativeLocation` (`self.InteractUI`) (`self.UILocation`) false false))

(fn `Interact`
  (params (Character :type "/Game/FirstPerson/Blueprints/FirstPersonCharacter Object Reference"))
  ;[1 1 1] Interaction
  (set `self.InteractionCharacter` Character)
  (`KismetSystemLibrary.PrintString` "Interacted"))

(fn `ToggleUI`
  (params (IsVisible :type Boolean))
  ;[1 1 1] Set UI Visibility
  (`SceneComponent.SetVisibility` (`self.InteractUI`) IsVisible false))

(fn `UserConstructionScript`
  ;[1 1 1] Construction - Init scripts
  (`self.InitMesh`)
  (`self.InitTrigger`)
  (`self.InitUI`))